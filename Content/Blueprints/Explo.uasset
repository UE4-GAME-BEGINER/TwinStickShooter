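; Explo is a short-lived explosion actor that damages characters caught in it.
; On BeginPlay it plays the explosion sound and particle effect at its location, then destroys itself after a brief delay.
; During that window, actor overlaps apply damage to living HeroCharacter or EnemyCharacter actors through AffectHealth, hurting enemies far more than heroes.
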(event `self.ReceiveBeginPlay`
  (bind (_returnvalue_location _returnvalue_rotation) (`KismetMathLibrary.BreakTransform` (`self.GetTransform`)))
  (`GameplayStatics.PlaySoundAtLocation` "/Game/StarterContent/Audio/Explosion_Cue.Explosion_Cue" _returnvalue_location (struct) 1.0 1.0 0.0 null null null)
  (`GameplayStatics.SpawnEmitterAtLocation` "/Game/StarterContent/Particles/P_Explosion.P_Explosion" _returnvalue_location _returnvalue_rotation)
  (`KismetSystemLibrary.Delay` 0.2)
  (`self.K2_DestroyActor`))

(event `self.ReceiveActorBeginOverlap`
  (params (OtherActor :type "Actor Object Reference"))
  (bind _ashero_character (cast `/Game/Blueprints/HeroCharacter` OtherActor)
    (:`then`
      (if (not (`MyCharacter.isDead` _ashero_character))
        (`/Game/Blueprints/HeroCharacter.Affect Health` _ashero_character -15.0)))
    (:`CastFailed`
      (bind _asenemy_character (cast `/Game/Blueprints/EnemyCharacter` OtherActor))
      (if (not (`MyCharacter.isDead` _asenemy_character))
        (`/Game/Blueprints/HeroCharacter.Affect Health` _asenemy_character -70.0)))))

(fn `UserConstructionScript`)