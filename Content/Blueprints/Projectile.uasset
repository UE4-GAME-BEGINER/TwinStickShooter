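; Projectile actor that damages non-player actors on overlap and destroys itself.
; On overlap, it sends an AffectHealthMessage with its Damage to actors that implement IDamagable and lack the Player tag, then spawns a Hit effect at its transform.
; Any other overlap, including a Player-tagged actor, spawns HitMetal instead and deals no damage.
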(event `self.ReceiveActorBeginOverlap`
  (params (OtherActor :type "Actor Object Reference"))
  (bind _returnvalue (`self.GetTransform`))
  (if (`KismetSystemLibrary.DoesImplementInterface` OtherActor "/Game/Blueprints/iDamagable.iDamagable_C")
    (if (not (`self.ActorHasTag` OtherActor "Player"))
      (message `/Game/Blueprints/iDamagable.Affect Health` OtherActor (`self.Damage`))
      (`|SpawnActorFromClass` "/Game/Blueprints/Hit.Hit_C" _returnvalue "Undefined" "OverrideRootScale" null null)
      (else
        (`|SpawnActorFromClass` "/Game/Blueprints/HitMetal.HitMetal_C" _returnvalue "Undefined" "OverrideRootScale" null null :!label _label)))
    (else
      (goto _label)))
  (`self.K2_DestroyActor`))

(fn `UserConstructionScript`)