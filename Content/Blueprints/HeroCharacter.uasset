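; Player hero for a twin-stick shooter that moves on world axes, faces the mouse's offset from screen center and fires an attached weapon.
; BeginPlay spawns the weapon on GunSocket, records the spawn transform in TwinStickMode and adds the HUD.
; AffectHealth handles death with a delayed explosion, then spends a life to respawn through the game mode or flags game over and quits.
; The construction script tints the body through a dynamic material.
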(event `/Game/Blueprints/iDamagable.Affect Health`
  (params (Delta :type "Float (single-precision)"))
  (bind _gamemode (`self.GameMode`))
  (bind _life (`/Game/Blueprints/TwinStickMode.life` _gamemode))
  (`self.CalculateHealth` Delta)
  (if (`self.isDead`)
    (`self.DisableInput` (`GameplayStatics.GetPlayerController` 0))
    (`/Game/Blueprints/Weapon.ReleaseTrigger` (`self.Weapon`))
    (`KismetSystemLibrary.Delay` 3.0)
    (`|SpawnActorFromClass` "/Game/Blueprints/Explo.Explo_C" (`self.GetTransform`) "Undefined" "OverrideRootScale" null null)
    (if (> _life 0)
      (set `/Game/Blueprints/TwinStickMode.life` (- _life 1) _gamemode)
      (`/Game/Blueprints/TwinStickMode.RespawnPlayer` _gamemode)
      (`self.K2_DestroyActor` (`self.Weapon`))
      (`self.K2_DestroyActor` self)
      (else
        (set `/Game/Blueprints/TwinStickMode.Gameover` true _gamemode)
        (`KismetSystemLibrary.Delay` 5.0)
        (`KismetSystemLibrary.QuitGame` null "Quit")))))

(event `self.ReceiveBeginPlay`
  (bind _mesh (`self.Mesh`))
  (`|ExecutionSequence`
    (:`then_0`
      (bind _returnvalue (`|SpawnActorFromClass` "/Game/Blueprints/Weapon.Weapon_C" (`SceneComponent.K2_GetComponentToWorld` _mesh) "Undefined" "OverrideRootScale" null null))
      (bind _output_get (set `self.Weapon` _returnvalue))
      (`self.K2_AttachToComponent` _output_get _mesh "GunSocket" "SnapToTarget" "SnapToTarget" "SnapToTarget" true))
    (:`then_1`
      (set `PlayerController.bShowMouseCursor` false (`GameplayStatics.GetPlayerController` 0)))
    (:`then_2`
      (bind _astwin_stick_mode (cast `/Game/Blueprints/TwinStickMode` (`GameplayStatics.GetGameMode`)))
      (bind _output_get_2 (set `self.GameMode` _astwin_stick_mode))
      (set `/Game/Blueprints/TwinStickMode.PlayerSpawnTransform` (`self.GetTransform`) _output_get_2))
    (:`then_3`
      (bind _returnvalue_2 (`|CreateWidget` "/Game/Blueprints/TwinStickHud.TwinStickHud_C"))
      (`UserWidget.AddToViewport` _returnvalue_2 0))))

(event `InputAction|FirebyPlayer`
  (params (Key :type "Key Structure"))
  (bind _weapon (`self.Weapon`))
  (:`Pressed`
    (`/Game/Blueprints/Weapon.PullTrigger` _weapon))
  (:`Released`
    (`/Game/Blueprints/Weapon.ReleaseTrigger` _weapon)))

(event `InputAxis|MoveUp`
  (params (AxisValue :type "Float (single-precision)"))
  ;[1 1 1] Movement
  (`self.AddMovementInput` (1.0 0.0 0.0) AxisValue))

(event `InputAxis|LookUp`
  (params (AxisValue :type "Float (single-precision)"))
  (bind (_x _y) (`KismetMathLibrary.BreakVector2D` (`WidgetLayoutLibrary.GetViewportSize`)))
  (bind (_locationx _locationy) (`PlayerController.GetMousePosition` (`GameplayStatics.GetPlayerController` 0)))
  ;[1 1 1] Rotation
  (`Controller.SetControlRotation` (`self.GetController`) (`KismetMathLibrary.MakeRotFromX` (`KismetMathLibrary.MakeVector` (+ (* (/ _locationy _y) -2.0) 1.0) (+ (* (/ _locationx _x) 2.0) -1.0))) :!label _label))

(event `InputAxis|LookRight`
  (params (AxisValue :type "Float (single-precision)"))
  ;[1 1 1] Rotation
  (goto _label))

(event `InputAxis|MoveRight`
  (params (AxisValue :type "Float (single-precision)"))
  ;[1 1 1] Movement
  (`self.AddMovementInput` (0.0 1.0 0.0) AxisValue))

(fn `UserConstructionScript`
  (bind _returnvalue (`PrimitiveComponent.CreateDynamicMaterialInstance` (`self.Mesh`) 0 null "None"))
  (bind _output_get (set `self.DynamicMat` _returnvalue))
  (`MaterialInstanceDynamic.SetVectorParameterValue` _output_get "BodyColor" (`self.HeroColor`)))