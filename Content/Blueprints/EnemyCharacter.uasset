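; Enemy character for a twin-stick game that damages the hero on contact and awards score when killed.
; Overlapping the hero starts a looping damage timer at AttacksPerSecond, cleared when the overlap ends.
; On death it ignores pawn collision, adds score, updates the saved high score in slot "1", emits smoke, then spawns Explo after a delay and destroys itself.
; The construction script tints the mesh with EnemyColor through a dynamic material.
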(event `/Game/Blueprints/iDamagable.Affect Health`
  (params (Delta :type "Float (single-precision)"))
  (bind (_returnvalue_location _returnvalue_rotation) (`KismetMathLibrary.BreakTransform` (`self.GetTransform`)))
  (bind _capsulecomponent (`self.CapsuleComponent`))
  (`self.CalculateHealth` Delta)
  (if (`self.isDead`)
    (`PrimitiveComponent.SetCollisionResponseToChannel` _capsulecomponent "ECC_WorldDynamic" "ECR_Ignore")
    (`PrimitiveComponent.SetCollisionResponseToChannel` _capsulecomponent "ECC_Pawn" "ECR_Ignore")
    (bind _astwin_stick_mode (cast `/Game/Blueprints/TwinStickMode` (`GameplayStatics.GetGameMode`)))
    (`/Game/Blueprints/TwinStickMode.IncrementScore` _astwin_stick_mode (`self.Delta Score`))
    (bind _returnvalue (`GameplayStatics.LoadGameFromSlot` "1"))
    (bind _asrecord (cast `/Game/Blueprints/record` _returnvalue)
      (:`then`
        (bind _score (`/Game/Blueprints/TwinStickMode.Score` _astwin_stick_mode))
        (if (> _score (`KismetMathLibrary.FTrunc` (`/Game/Blueprints/record.score` _asrecord)))
          (set `/Game/Blueprints/record.score` (`KismetMathLibrary.Conv_IntToDouble` _score) _asrecord)))
      (:`CastFailed`
        _))
    (`GameplayStatics.SaveGameToSlot` _asrecord "1")
    (bind _returnvalue_2 (`GameplayStatics.LoadGameFromSlot` "1"))
    (bind _asrecord_2 (cast `/Game/Blueprints/record` _returnvalue_2))
    (set `/Game/Blueprints/TwinStickMode.HighestScore` (`/Game/Blueprints/record.score` _asrecord_2) _astwin_stick_mode)
    (`GameplayStatics.SpawnEmitterAtLocation` "/Game/StarterContent/Particles/BrokenSmoke.BrokenSmoke" (- (- _returnvalue_location (* (`KismetMathLibrary.Normal` (`KismetMathLibrary.GetForwardVector` _returnvalue_rotation)) (`self.smoke_loc`))) (0.0 0.0 100.0)) _returnvalue_rotation)
    (`self.DetachFromControllerPendingDestroy`)
    (`KismetSystemLibrary.Delay` 3.0)
    (`|SpawnActorFromClass` "/Game/Blueprints/Explo.Explo_C" (`self.GetTransform`) "Undefined" "OverrideRootScale" null null)
    (`self.K2_DestroyActor`)))

(event `self.ReceiveActorBeginOverlap`
  (params (OtherActor :type "Actor Object Reference"))
  (bind _ashero_character (cast `/Game/Blueprints/HeroCharacter` OtherActor))
  (set `self.Hero` _ashero_character)
  (`/Engine/EditorBlueprintResources/StandardMacros.DoOnce` false :!label _label
    (:`Completed`
      (`self.DamageTheHero`)
      (`KismetSystemLibrary.K2_SetTimer` null "DamageTheHero" (/ 1.0 (`self.AttacksPerSecond`)) true))))

(event `self.ReceiveActorEndOverlap`
  (params (OtherActor :type "Actor Object Reference"))
  (if (== OtherActor (`self.Hero`))
    (`KismetSystemLibrary.K2_ClearTimer` null "DamageTheHero")
    (goto _label :!via `Reset`)))

(event `DamageTheHero`
  (`/Game/Blueprints/HeroCharacter.Affect Health` (`self.Hero`) (`self.Damage`)))

(fn `UserConstructionScript`
  (bind _returnvalue (`PrimitiveComponent.CreateDynamicMaterialInstance` (`self.Mesh`) 0 null "None"))
  (bind _output_get (set `self.dyna mat` _returnvalue))
  (`MaterialInstanceDynamic.SetVectorParameterValue` _output_get "BodyColor" (`self.EnemyColor`)))